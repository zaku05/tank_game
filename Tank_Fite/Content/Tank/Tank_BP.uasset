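; Player-controllable tank pawn that wires components and input for driving, aiming and firing.
; BeginPlay passes the barrel and turret to their setters and both tracks to TankMovement.
; Input drives either each track's throttle directly or forward and turn intents through TankMovement, while Fire calls the fire function.
; Frame-time-scaled aim input yaws SpringArm for azimuth and pitches AzimuthGimbal for elevation, despite the latter's name.
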(event EventBeginPlay
  (Class|Tank|SetBarrelReference (Variables|Default|GetBarrel))
  (Class|Tank|SetTurretReference (Variables|Default|GetTankTurretSM))
  (Class|TankMovementComponent|Initialize (Variables|Default|GetTankMovement) (Variables|Default|GetLeftTankTrack) (Variables|Default|GetRightTankTrack)))

(event Input|ActionEvents|InputActionFire
  (params (Key :type Key%20Structure))
  ;[1 1 1] Aim Input binding
  (:Pressed
    (Class|Tank|Fire)))

(event Input|AxisEvents|InputAxisAim_Azimuth
  (params (AxisValue :type Float%20%28single-precision%29))
  ;[1 1 1] Aim Input binding
  (Transformation|AddLocalRotation (Variables|Default|GetSpringArm) (Math|Rotator|MakeRotator 0.0 0.0 (* AxisValue (Utilities|Time|GetWorldDeltaSeconds) 1e+02)) false false))

(event Input|AxisEvents|InputAxisLeftTrackThrottle
  (params (AxisValue :type Float%20%28single-precision%29))
  ;[1 1 1] Movement Input Binding
  (Class|TankTrack|SetThrottle (Variables|Default|GetLeftTankTrack) AxisValue))

(event Input|AxisEvents|InputAxisRightTrackThrottle
  (params (AxisValue :type Float%20%28single-precision%29))
  ;[1 1 1] Movement Input Binding
  (Class|TankTrack|SetThrottle (Variables|Default|GetRightTankTrack) AxisValue))

(event Input|AxisEvents|InputAxisAim_Elevation
  (params (AxisValue :type Float%20%28single-precision%29))
  ;[1 1 1] Aim Input binding
  (Transformation|AddLocalRotation (Variables|Default|Getazimuth%20gimbal) (Math|Rotator|MakeRotator 0.0 (* AxisValue (Utilities|Time|GetWorldDeltaSeconds) 1e+02) 0.0) false false))

(event Input|AxisEvents|InputAxisMoveForward
  (params (AxisValue :type Float%20%28single-precision%29))
  ;[1 1 1] Movement Input Binding
  (Class|TankMovementComponent|IntendMoveForward (Variables|Default|GetTankMovement) AxisValue))

(event Input|AxisEvents|InputAxisTurning
  (params (AxisValue :type Float%20%28single-precision%29))
  ;[1 1 1] Movement Input Binding
  (Class|TankMovementComponent|IntendTurnRight (Variables|Default|GetTankMovement) AxisValue))

(fn ConstructionScript)